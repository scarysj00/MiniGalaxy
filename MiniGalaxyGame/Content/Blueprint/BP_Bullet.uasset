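; BP_Bullet is a projectile actor that flies straight along its forward vector and destroys any BP_Enemy it overlaps.
; Tick calls a Translate helper that offsets the location by normalized direction, Speed and delta seconds, without sweeping.
; On overlapping a BP_Enemy, it spawns a particle effect at the enemy, destroys both actors and plays a 2D explosion sound.
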(event `self.ReceiveActorBeginOverlap`
  (params (OtherActor :type "Actor Object Reference"))
  (bind _asbp_enemy (cast `/Game/Blueprint/BP_Enemy` OtherActor))
  (`GameplayStatics.SpawnEmitterAtLocation` "/Engine/Tutorial/SubEditors/TutorialAssets/TutorialParticleSystem.TutorialParticleSystem" (`self.K2_GetActorLocation` _asbp_enemy))
  (`self.K2_DestroyActor` _asbp_enemy)
  (`self.K2_DestroyActor`)
  (`GameplayStatics.PlaySound2D` "/Game/Resource/explosion_sound.explosion_sound" 1.0 1.0 0.0 null null))

(event `self.ReceiveBeginPlay`)

(event `self.ReceiveTick`
  (params (DeltaSeconds :type "Float (single-precision)"))
  ; 나의 전방 방향으로 이동하고 싶다. P = P0 + VT
  (`self.Translate` (`self.GetActorForwardVector`) (`self.Speed`)))

(fn `Translate`
  (params (Direction :type "Vector Structure") (Speed :type "Float (double-precision)") (Sweep :type Boolean))
  (`self.K2_SetActorLocation` (+ (`self.K2_GetActorLocation`) (* (`KismetMathLibrary.Normal` Direction) Speed (`GameplayStatics.GetWorldDeltaSeconds`))) Sweep))

(fn `UserConstructionScript`)