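; BP_Enemy is a shoot-'em-up style enemy that picks a heading on spawn and flies straight along it.
; On BeginPlay it has a 30% chance to aim at the player's current position, otherwise it uses its own forward vector.
; Tick moves it through a Translate helper at a frame-rate-independent speed.
; Overlapping BP_Player spawns an explosion effect, destroys both actors and plays a sound.
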(event `self.ReceiveBeginPlay`
  ; 적이 생성될 때(BeginPlay) 방향을 30% 확률로 플레이어를 향하는 방향과 나머지 확률은 아래로 떨어지는 방향으로 정하고, 살아가면서(Tick) 계속 이 확률로 이동하고 싶다.
  (if (< (`KismetMathLibrary.RandomIntegerInRange` 0 9) 3)
    (set `self.Direction` (`KismetMathLibrary.Normal` (- (`self.K2_GetActorLocation` (`GameplayStatics.GetPlayerPawn` 0)) (`self.K2_GetActorLocation`))))
    (else
      (set `self.Direction` (`self.GetActorForwardVector`)))))

(event `self.ReceiveTick`
  (params (DeltaSeconds :type "Float (single-precision)"))
  (`self.Translate` (`self.Direction`) (`self.Speed`)))

(event `self.ReceiveActorBeginOverlap`
  (params (OtherActor :type "Actor Object Reference"))
  (bind _asbp_player (cast `/Game/Blueprint/BP_Player` OtherActor))
  (`GameplayStatics.SpawnEmitterAtLocation` "/Engine/Tutorial/SubEditors/TutorialAssets/TutorialParticleSystem.TutorialParticleSystem" (`self.K2_GetActorLocation` _asbp_player))
  (`self.K2_DestroyActor` _asbp_player)
  (`self.K2_DestroyActor`)
  (`GameplayStatics.PlaySound2D` "/Game/Resource/explosion_sound.explosion_sound" 1.0 1.0 0.0 null null))

(fn `Translate`
  (params (Direction :type "Vector Structure") (Speed :type "Float (double-precision)") (Sweep :type Boolean))
  (`self.K2_SetActorLocation` (+ (`self.K2_GetActorLocation`) (* (`KismetMathLibrary.Normal` Direction) Speed (`GameplayStatics.GetWorldDeltaSeconds`))) Sweep))

(fn `UserConstructionScript`)